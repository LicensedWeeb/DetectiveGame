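; BP_CameraPoint is a room trigger that repositions the top-down character's camera and toggles room fog.
; When the player overlaps its Box, or at BeginPlay if marked IsStart, it sets the character's CamPos to its Arrow and calls MoveCamera.
; ToggleFog flips its own Fog visibility on entry and exit, along with that of ConnectedRooms when IsConnected is set.
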(event `self.ReceiveBeginPlay`
  (if (`self.isStart`)
    (bind _asbp_top_down_character (cast `/Game/TopDown/Blueprints/BP_TopDownCharacter` (`GameplayStatics.GetPlayerPawn` 0)))
    (set `/Game/TopDown/Blueprints/BP_TopDownCharacter.camPos` (`self.Arrow`) _asbp_top_down_character)
    (`/Game/TopDown/Blueprints/BP_TopDownCharacter.Move Camera` _asbp_top_down_character)
    (`self.ToggleFog`)))

(event `self.Box.OnComponentBeginOverlap`
  (params (OverlappedComponent :type "PrimitiveComponent Object Reference") (OtherActor :type "Actor Object Reference") (OtherComp :type "PrimitiveComponent Object Reference") (OtherBodyIndex :type Integer) (bFromSweep :type Boolean) (SweepResult :type "HitResult Structure (by ref)"))
  (if (`self.ActorHasTag` OtherActor "Player")
    (bind _asbp_top_down_character (cast `/Game/TopDown/Blueprints/BP_TopDownCharacter` OtherActor))
    (set `/Game/TopDown/Blueprints/BP_TopDownCharacter.camPos` (`self.Arrow`) _asbp_top_down_character)
    (`/Game/TopDown/Blueprints/BP_TopDownCharacter.Move Camera` _asbp_top_down_character)
    (`self.ToggleFog`)))

(event `self.Box.OnComponentEndOverlap`
  (params (OverlappedComponent :type "PrimitiveComponent Object Reference") (OtherActor :type "Actor Object Reference") (OtherComp :type "PrimitiveComponent Object Reference") (OtherBodyIndex :type Integer))
  (if (`self.ActorHasTag` OtherActor "Player")
    (`self.ToggleFog`)))

(event `ToggleFog`
  (bind _connectedrooms (`self.connectedRooms`))
  (if (`self.isConnected`)
    (for _index (range (+ (`KismetArrayLibrary.Array_Length` _connectedrooms) 1))
      (bind _fog (`/Game/Characters/BP_CameraPoint.Fog` (`|GetArrayItem` _connectedrooms _index)))
      (`/Engine/EditorBlueprintResources/StandardMacros.IsValid` _fog
        (:`Is Valid`
          (`SceneComponent.ToggleVisibility` _fog false))))
    (`SceneComponent.ToggleVisibility` (`self.Fog`) false)
    (else
      (`SceneComponent.ToggleVisibility` (`self.Fog`) false))))

(fn `UserConstructionScript`)