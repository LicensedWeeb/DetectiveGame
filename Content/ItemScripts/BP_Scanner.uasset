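; BP_Scanner is a one-shot scan pulse that highlights past or present items it touches.
; On BeginPlay, a timeline scales the actor and drives the sphere material's opacity, then disables collision and hides the actor.
; Each overlap loops over all BP_Item_Past actors, using their IsPastActive flags to choose whether to cast the overlapped actor to BP_Item_Past or BP_Item_Present and highlight it.
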(event `self.Sphere.OnComponentBeginOverlap`
  (params (OverlappedComponent :type "PrimitiveComponent Object Reference") (OtherActor :type "Actor Object Reference") (OtherComp :type "PrimitiveComponent Object Reference") (OtherBodyIndex :type Integer) (bFromSweep :type Boolean) (SweepResult :type "HitResult Structure (by ref)"))
  ; Highlights past or present items depending on if the player is in the past or present
  (bind _outactors (`GameplayStatics.GetAllActorsOfClass` "/Game/ItemScripts/BP_Item_Past.BP_Item_Past_C"))
  (for _array_element _outactors
    (if (`/Game/ItemScripts/BP_Item_Past.IsPastActive` _array_element)
      (bind _asbp_item_past (cast `/Game/ItemScripts/BP_Item_Past` OtherActor))
      (`/Game/ItemScripts/BP_Item_Past.Highlight` _asbp_item_past)
      (else
        (bind _asbp_item_present (cast `/Game/ItemScripts/BP_Item_Present` OtherActor))
        (`/Game/ItemScripts/BP_Item_Present.Highlight` _asbp_item_present)))))

(event `self.ReceiveBeginPlay`
  ; Handles the animation and collision detection of the scan
  (`self.Do Scan`))

(event `Do Scan`
  ; Handles the animation and collision detection of the scan
  (`PrimitiveComponent.SetCollisionEnabled` (`self.Sphere`) "QueryOnly")
  (bind (_direction _scannerexpandsize _scanneropacity) (`Timeline|Timeline` :!via `PlayFromStart`)
    (:`Update`
      (`self.SetActorScale3D` (`KismetMathLibrary.Conv_DoubleToVector` _scannerexpandsize))
      (`MeshComponent.SetScalarParameterValueOnMaterials` (`self.Sphere`) "Scanner_Opacity" _scanneropacity))
    (:`Finished`
      (`PrimitiveComponent.SetCollisionEnabled` (`self.Sphere`) "NoCollision")
      (`self.SetActorHiddenInGame` true))))

(fn `UserConstructionScript`)