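; BP_CorpseItem is an interactable corpse item that unlocks NPC questions and advances an ordered item sequence.
; When Interact fires while it is collectable, it increments TotalQuestions on each valid NPC in EffectedNPCs.
; It then advances the AllItems index, makes the item at that index collectable and clears its own collectable flag.
; An older PastList-based advance remains in the graph but never runs.
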(event `/Game/TopDown/Blueprints/InteractInterface.Interact`
  (bind _allitems (`self.allItems`))
  (bind _effectednpcs (`self.effectedNPCs`))
  ; Loops through each effected npc and makes next question available when its a past item
  (if (`self.isCollectable`)
    (for _index (range (+ (`KismetArrayLibrary.Array_Length` _effectednpcs) 1))
      (bind _output (`|GetArrayItem` _effectednpcs _index))
      (`/Engine/EditorBlueprintResources/StandardMacros.IsValid` _output
        (:`Is Valid`
          (set `/Game/AI/NPC_AI.totalQuestions` (+ (`/Game/AI/NPC_AI.totalQuestions` _output) 1) _output))))
    (bind _output_get (set `/Game/ItemScripts/AllItems.CurrentItem` (+ (`/Game/ItemScripts/AllItems.CurrentItem` _allitems) 1) _allitems))
    (bind _output_2 (`|GetArrayItem` (`/Game/ItemScripts/AllItems.Items` _allitems) _output_get))
    (`/Engine/EditorBlueprintResources/StandardMacros.IsValid` _output_2
      (:`Is Valid`
        (set `/Game/ItemScripts/ItemBP.isCollectable` true _output_2))
      (:`Is Not Valid`
        _))
    (set `self.isCollectable` false)))

(fn `UserConstructionScript`
  (`parent.UserConstructionScript`))