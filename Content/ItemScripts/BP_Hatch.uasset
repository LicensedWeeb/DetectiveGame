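; BP_Hatch is a hatch that teleports the top-down player when they press F inside its box, gated on AllItems.CurrentItem reaching a threshold.
; Box overlaps store or clear the player, while Tick polls the key and item state.
; The teleport moves the player to the Arrow's transform, aligns control rotation, zeroes velocity and clears the reference.
; The construction script places the Arrow from the TeleportLocation variable.
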(event `self.ReceiveBeginPlay`
  (bind _returnvalue (`GameplayStatics.GetActorOfClass` "/Game/ItemScripts/AllItems.AllItems_C"))
  (set `self.All Items` _returnvalue))

(event `self.ReceiveTick`
  (params (DeltaSeconds :type "Float (single-precision)"))
  (bind _player (`self.Player`))
  (bind _player_2 (`self.Player`))
  (bind (_returnvalue_location _returnvalue_rotation) (`KismetMathLibrary.BreakTransform` (`SceneComponent.K2_GetComponentToWorld` (`self.Arrow`))))
  ; Teleport the stupid chud player
  (`/Engine/EditorBlueprintResources/StandardMacros.IsValid` _player
    (:`Is Valid`
      (if (and (>= (`/Game/ItemScripts/AllItems.CurrentItem` (`self.All Items`)) 11) (`PlayerController.IsInputKeyDown` (`GameplayStatics.GetPlayerController` 0) "F"))
        (`SceneComponent.K2_SetWorldTransform` (`Actor.RootComponent` _player) (`KismetMathLibrary.MakeTransform` _returnvalue_location _returnvalue_rotation) false false)
        (`Controller.SetControlRotation` (`GameplayStatics.GetPlayerController` 0) (`self.K2_GetActorRotation` _player_2))
        (set `MovementComponent.Velocity` (0.0 0.0 0.0) (`Character.CharacterMovement` _player_2))
        (set `self.Player` null)))))

(event `self.Box.OnComponentBeginOverlap`
  (params (OverlappedComponent :type "PrimitiveComponent Object Reference") (OtherActor :type "Actor Object Reference") (OtherComp :type "PrimitiveComponent Object Reference") (OtherBodyIndex :type Integer) (bFromSweep :type Boolean) (SweepResult :type "HitResult Structure (by ref)"))
  (bind _asbp_top_down_character (cast `/Game/TopDown/Blueprints/BP_TopDownCharacter` OtherActor))
  (set `self.Player` _asbp_top_down_character))

(event `self.Box.OnComponentEndOverlap`
  (params (OverlappedComponent :type "PrimitiveComponent Object Reference") (OtherActor :type "Actor Object Reference") (OtherComp :type "PrimitiveComponent Object Reference") (OtherBodyIndex :type Integer))
  (cast `/Game/TopDown/Blueprints/BP_TopDownCharacter` OtherActor)
  (set `self.Player` null))

(fn `UserConstructionScript`
  (`SceneComponent.K2_SetRelativeTransform` (`self.Arrow`) (`self.TeleportLocation`) false false))