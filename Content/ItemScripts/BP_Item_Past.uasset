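; BP_Item_Past is an item actor for a past/present mechanic, with a highlightable Cube mesh.
; Every Tick it reads IsPastActive and shows or hides all valid actors in PastItems, toggling their collision to match.
; A hit on the Cube applies an outline overlay material, and ending an actor overlap clears it.
; The Highlight event applies a separate highlight overlay for a short delay, then removes it.
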(event `self.Cube.OnComponentHit`
  (params (HitComponent :type "PrimitiveComponent Object Reference") (OtherActor :type "Actor Object Reference") (OtherComp :type "PrimitiveComponent Object Reference") (NormalImpulse :type "Vector Structure") (Hit :type "HitResult Structure (by ref)"))
  ; Highlight interactable objects
  (`MeshComponent.SetOverlayMaterial` (`self.Cube`) "/Game/Materials/OutlineMaterial.OutlineMaterial"))

(event `self.ReceiveActorEndOverlap`
  (params (OtherActor :type "Actor Object Reference"))
  ; Highlight interactable objects
  (`MeshComponent.SetOverlayMaterial` (`self.Cube`) null))

(event `Highlight`
  ; Function to highlight the interactable materials
  (`MeshComponent.SetOverlayMaterial` (`self.Cube`) "/Game/Materials/M_HighlightItem.M_HighlightItem")
  (`KismetSystemLibrary.Delay` 2.0)
  (`MeshComponent.SetOverlayMaterial` (`self.Cube`) null))

(event `self.ReceiveTick`
  (params (DeltaSeconds :type "Float (single-precision)"))
  (bind _pastitems (`self.PastItems`))
  ; Checks to see if present or past is active and hides the past items if present is active
  (if (`self.IsPastActive`)
    (for _array_element _pastitems
      (`/Engine/EditorBlueprintResources/StandardMacros.IsValid` _array_element
        (:`Is Valid`
          (`self.SetActorHiddenInGame` _array_element false)
          (`self.SetActorEnableCollision` _array_element true))))
    (else
      (for _array_element_2 _pastitems
        (`/Engine/EditorBlueprintResources/StandardMacros.IsValid` _array_element_2
          (:`Is Valid`
            (`self.SetActorHiddenInGame` _array_element_2 true)
            (`self.SetActorEnableCollision` _array_element_2 false)))))))

(fn `UserConstructionScript`)